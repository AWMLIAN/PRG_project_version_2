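; Quest component that tracks the active quest's objectives and drives the quest HUD.
; It creates a hidden WB_QuestHUD widget on BeginPlay, then fills it with the quest name and objectives.
; Enemy-elimination and chest-opening events update matching objective structs by reference, mark finished ones completed and update the HUD.
; A completion counter clears the quest and plays the HUD's completion animation once all objectives are done.
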(event Custom|Set%20Active%20Quest%20Text
  (Rendering|Components|TextRender|SetText (Variables|/Game/Quest_System/WB_QuestHUD.WB_QuestHUD_C|GetActiveQuestText (Variables|Default|GetQuestHUD%20Widget)) (Utilities|Text|ToText(String) (.Name (Utilities|Struct|BreakS_Quest (Variables|Default|GetActiveQuest)))))
  (Default|ShowQuestPanel (Variables|Default|GetQuestHUD%20Widget)))

(event Custom|Set%20Objective
  (Default|FillObjectives (Variables|Default|GetQuestHUD%20Widget) (.objective (Variables|Default|GetActiveQuest))))

(event Custom|Eliminate%20Enemy
  (params (Enemy%20Eliminated :type Actor%20Object%20Reference))
  (for _array_element (.objective (Variables|Default|GetActiveQuest))
    (if (and (not (.Completed (Utilities|Struct|BreakS_QuestObjective _array_element))) (.IsEliminateEnemyObjective (Utilities|Struct|BreakS_QuestObjective _array_element)))
      (if (!= (Utilities|Array|Length (Variables|Default|Getenemy%20actors%20array)) 0)
        _
        (else
          (bind _output_get (Variables|Default|Setenemy%20actors%20array (.ActorToEliminate (Utilities|Struct|BreakS_QuestObjective _array_element))))))
      (Utilities|Array|RemoveItem _output_get Enemy%20Eliminated)
      (|SetBy-RefVar _array_element (Utilities|Struct|MakeS_QuestObjective (.NameAim (Utilities|Struct|BreakS_QuestObjective _array_element)) false (Variables|Default|Getenemy%20actors%20array) (.ChestToOpen (Utilities|Struct|BreakS_QuestObjective _array_element)) (.IsEliminateEnemyObjective (Utilities|Struct|BreakS_QuestObjective _array_element)) (.IsChestObjective (Utilities|Struct|BreakS_QuestObjective _array_element))))
      (Development|PrintString (Utilities|String|ToString(Integer) (Utilities|Array|Length (Variables|Default|Getenemy%20actors%20array))))
      (if (== (Utilities|Array|Length (Variables|Default|Getenemy%20actors%20array)) 0)
        (|SetBy-RefVar _array_element (Utilities|Struct|MakeS_QuestObjective (.NameAim (Utilities|Struct|BreakS_QuestObjective _array_element)) true 0 (.ChestToOpen (Utilities|Struct|BreakS_QuestObjective _array_element)) (.IsEliminateEnemyObjective (Utilities|Struct|BreakS_QuestObjective _array_element)) (.IsChestObjective (Utilities|Struct|BreakS_QuestObjective _array_element))))
        (Default|CompleteObjective (Variables|Default|GetQuestHUD%20Widget) _array_element)
        (CallFunction|ObjectiveCompleted)
        (Development|PrintText "Complete!")))))

(event Custom|Open%20Chest
  (params (Chest :type Actor%20Object%20Reference))
  (for _array_element (.objective (Variables|Default|GetActiveQuest))
    (if (and (.IsChestObjective (Utilities|Struct|BreakS_QuestObjective _array_element)) (== Chest (.ChestToOpen (Utilities|Struct|BreakS_QuestObjective _array_element))))
      (|SetBy-RefVar _array_element (Utilities|Struct|MakeS_QuestObjective (.NameAim (Utilities|Struct|BreakS_QuestObjective _array_element)) true (.ActorToEliminate (Utilities|Struct|BreakS_QuestObjective _array_element)) 0 (.IsEliminateEnemyObjective (Utilities|Struct|BreakS_QuestObjective _array_element)) (.IsChestObjective (Utilities|Struct|BreakS_QuestObjective _array_element))))
      (Default|CompleteObjective (Variables|Default|GetQuestHUD%20Widget) _array_element)
      (CallFunction|ObjectiveCompleted)
      (Development|PrintText "Complete!"))))

(event Custom|Objective%20Completed
  (Math|Integer|IncrementInt (Variables|Default|GetobjectivesCompletded)
    (:%20%20
      (if (>= (Variables|Default|GetobjectivesCompletded) (Utilities|Array|Length (.objective (Variables|Default|GetActiveQuest))))
        (Development|PrintString "QUEST COMPLETED")
        (Variables|Default|SetActiveQuest "")
        (Variables|Default|SetobjectivesCompletded 0)
        (Default|PlayQuestCompletedAnimation (Variables|Default|GetQuestHUD%20Widget))))))

(event EventBeginPlay
  (bind _returnvalue (UserInterface|CreateWidget "/Game/Quest_System/WB_QuestHUD.WB_QuestHUD_C"))
  (bind _output_get (Variables|Default|SetQuestHUD%20Widget _returnvalue))
  (UserInterface|Viewport|AddtoViewport _output_get 0)
  (Default|HideQuestPanel (Variables|Default|GetQuestHUD%20Widget)))