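; BP_QuestGiver is an NPC-style actor that plays dialogue, then offers its list of quests to the player.
; An interact widget turns to face the camera and shows only while the third-person character is inside the trigger radius.
; Each Interact advances the Dialogue array, then opens a WB_QuestGiver widget filled from Quests.
; Interacting again or calling CloseWidget removes that widget and restores game-only input.
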(event OnComponentBeginOverlap(TriggerRadius)
  (params (OverlappedComponent :type Primitive%20Component%20Object%20Reference) (OtherActor :type Actor%20Object%20Reference) (OtherComp :type Primitive%20Component%20Object%20Reference) (OtherBodyIndex :type Integer) (bFromSweep :type Boolean) (SweepResult :type Hit%20Result%20Structure%20%28by%20ref%29))
  (Utilities|Casting|CastToBP_ThirdPersonCharacter OtherActor)
  (Rendering|SetVisibility (Variables|Default|GetInteract%20Widget) true false))

(event OnComponentEndOverlap(TriggerRadius)
  (params (OverlappedComponent :type Primitive%20Component%20Object%20Reference) (OtherActor :type Actor%20Object%20Reference) (OtherComp :type Primitive%20Component%20Object%20Reference) (OtherBodyIndex :type Integer))
  (Utilities|Casting|CastToBP_ThirdPersonCharacter OtherActor)
  (Rendering|SetVisibility (Variables|Default|GetInteract%20Widget) false false))

(event Custom|Close%20Widget
  (bind _returnvalue (Game|GetPlayerController 0))
  (Widget|RemovefromParent (Variables|Default|GetQuest%20Widget))
  (Variables|Default|SetQuest%20Widget 0)
  (Variables|/Script/Engine.PlayerController|SetbShowMouseCursor _returnvalue false)
  (Input|SetInputModeGameOnly _returnvalue false)
  (Variables|Default|SetWidgetActivated false))

(event Custom|Open%20QuestWidget
  (Development|PrintText "Giving quest!")
  (bind _returnvalue (UserInterface|CreateWidget "/Game/Quest_System/WB_QuestGiver.WB_QuestGiver_C"))
  (bind _output_get (Variables|Default|SetQuest%20Widget _returnvalue))
  (UserInterface|Viewport|AddtoViewport _output_get 0)
  (Variables|Default|SetWidgetActivated true)
  (Variables|/Game/Quest_System/WB_QuestGiver.WB_QuestGiver_C|SetQuestGiverBP (Variables|Default|GetQuest%20Widget) self)
  (for _array_element (Variables|Default|GetQuests)
    (Default|AddQuest (Variables|Default|GetQuest%20Widget) _array_element)))

(event EventInteract
  (bind _returnvalue (Game|GetPlayerController 0))
  (bind _returnvalue_2 (Game|GetPlayerController 0))
  (if (not (Variables|Default|GetWidgetActivated))
    (if (not (Variables|Default|GetDialogueOpened))
      (bind _returnvalue_3 (UserInterface|CreateWidget "/Game/Quest_System/WB_QuestGiverDialogue.WB_QuestGiverDialogue_C"))
      (bind _output_get (Variables|Default|SetDialogueWidget _returnvalue_3))
      (UserInterface|Viewport|AddtoViewport _returnvalue_3 0)
      (Variables|Default|SetDialogueOpened true)
      (Rendering|Components|TextRender|SetText (Variables|/Game/Quest_System/WB_QuestGiverDialogue.WB_QuestGiverDialogue_C|GetDialogueText (Variables|Default|GetDialogueWidget)) (Utilities|Text|ToText(String) (Utilities|Array|Get(acopy) (Variables|Default|GetDialogue) (Variables|Default|GetDialogueIndex))))
      (Math|Integer|IncrementInt (Variables|Default|GetDialogueIndex)
        (:%20%20
          (Variables|/Script/Engine.PlayerController|SetbShowMouseCursor _returnvalue_2 true)
          (Input|SetInputModeGameandUI _returnvalue_2 (Variables|Default|GetQuest%20Widget) "DoNotLock" true false)))
      (else
        (Rendering|Components|TextRender|SetText (Variables|/Game/Quest_System/WB_QuestGiverDialogue.WB_QuestGiverDialogue_C|GetDialogueText (Variables|Default|GetDialogueWidget)) (Utilities|Text|ToText(String) (Utilities|Array|Get(acopy) (Variables|Default|GetDialogue) (Variables|Default|GetDialogueIndex))))
        (Math|Integer|IncrementInt (Variables|Default|GetDialogueIndex)
          (:%20%20
            (if (> (Variables|Default|GetDialogueIndex) (Utilities|Array|Length (Variables|Default|GetDialogue)))
              (Widget|RemovefromParent (Variables|Default|GetDialogueWidget))
              (Variables|Default|SetDialogueWidget 0)
              (Variables|Default|SetDialogueIndex 0)
              (Variables|Default|SetDialogueOpened false)
              (CallFunction|OpenQuestWidget))))))
    (else
      (Widget|RemovefromParent (Variables|Default|GetQuest%20Widget))
      (Variables|Default|SetQuest%20Widget 0)
      (Variables|/Script/Engine.PlayerController|SetbShowMouseCursor _returnvalue false)
      (Input|SetInputModeGameOnly _returnvalue false)
      (Variables|Default|SetWidgetActivated false))))

(event EventTick
  (params (DeltaSeconds :type Float%20%28single-precision%29))
  (Transformation|SetWorldRotation (Variables|Default|GetInteract%20Widget) (Math|Rotator|FindLookatRotation (Transformation|GetWorldLocation (Variables|Default|GetInteract%20Widget)) (Transformation|GetWorldLocation (Variables|/Script/Engine.PlayerCameraManager|GetTransformComponent (Game|GetPlayerCameraManager 0)))) false false))

(fn ConstructionScript)