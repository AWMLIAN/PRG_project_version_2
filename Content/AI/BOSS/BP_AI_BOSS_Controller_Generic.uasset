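; Generic boss AI controller that runs the BT_AI_BOSS behavior tree on BeginPlay and manages the boss health bar.
; ActivateBossCombat creates a WB_BOSSHealthBar widget and adds it to the viewport, and DeactivateBossCombat removes it and clears the reference.
; While the widget is valid, Tick sets its bar to the ratio of Health to MaxHealth, polling every frame.
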(event Custom|Activate%20BossCombat
  (bind _returnvalue (UserInterface|CreateWidget "/Game/UI/WB_BOSSHealthBar.WB_BOSSHealthBar_C"))
  (bind _output_get (Variables|Default|SetBossHealthBarWidget _returnvalue))
  (UserInterface|Viewport|AddtoViewport _output_get 0))

(event Custom|Deactivate%20BossCombat
  (Widget|RemovefromParent (Variables|Default|GetBossHealthBarWidget))
  (Variables|Default|SetBossHealthBarWidget 0))

(event EventBeginPlay
  (AI|RunBehaviorTree "/Game/AI/BOSS/BT_AI_BOSS.BT_AI_BOSS"))

(event EventTick
  (params (DeltaSeconds :type Float%20%28single-precision%29))
  (bind _bosshealthbarwidget (Variables|Default|GetBossHealthBarWidget)
    (:then
      (Progress|SetPercent (Variables|/Game/UI/WB_BOSSHealthBar.WB_BOSSHealthBar_C|GetHealthBar _bosshealthbarwidget) (/ (Variables|Default|GetHealth) (Variables|Default|GetMaxHealth))))
    (:else)))

(fn ConstructionScript
  (|CallParentFunction))