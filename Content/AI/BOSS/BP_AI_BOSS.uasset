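; BP_AI_BOSS is a boss AI Blueprint that passes its health to its AI controller.
; Each Tick, after the parent Tick, it casts its controller to BP_AI_BOSS_Controller_Generic and copies CurrentHealth and MaxHealth from BPCPlayerState into it.
; BeginPlay and overlap events are disabled or empty, and the construction script only calls its parent.
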(event EventBeginPlay
  (|CallParentFunction) ; 此节点被禁用，将不会被调用。\n从引脚连出引线来编译功能。
)

(event Collision|EventActorBeginOverlap
  (params (OtherActor :type Actor%20Object%20Reference)))

(event EventTick
  (params (DeltaSeconds :type Float%20%28single-precision%29))
  (bind _bpc_playerstate (Variables|Default|GetBPC_playerState))
  (|CallParentFunction DeltaSeconds)
  (bind _asbp_ai_boss_controller_generic (Utilities|Casting|CastToBP_AI_BOSS_Controller_Generic (AI|GetAIController self)))
  (Variables|/Game/AI/BOSS/BP_AI_BOSS_Controller_Generic.BP_AI_BOSS_Controller_Generic_C|SetHealth _asbp_ai_boss_controller_generic (Variables|/Game/BluePrints/BPC_playerState.BPC_playerState_C|GetCurrent%20Health _bpc_playerstate))
  (Variables|/Game/AI/BOSS/BP_AI_BOSS_Controller_Generic.BP_AI_BOSS_Controller_Generic_C|SetMaxHealth _asbp_ai_boss_controller_generic (Variables|/Game/BluePrints/BPC_playerState.BPC_playerState_C|GetMax%20Health _bpc_playerstate)))

(fn ConstructionScript
  (|CallParentFunction))