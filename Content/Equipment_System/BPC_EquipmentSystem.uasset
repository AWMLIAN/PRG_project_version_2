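; Actor component for the third-person character that handles weapon pickup and the equipment menu.
; Interact input sphere-traces from the follow camera, stores the hit BP_Weapon's item data in WeaponSlots and destroys the actor.
; The menu input toggles a lazily created, reused WB_Equipment widget, switching cursor and input mode while disabling attacks and movement when open.
; A debug key prints the stored weapon row names.
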(event Input|EnhancedActionEvents|EnhancedInputActionIA_Interact
  (params (ActionValue :type Boolean) (ElapsedSeconds :type Float%20%28double-precision%29) (TriggeredSeconds :type Float%20%28double-precision%29) (InputAction :type Input%20Action%20Object%20Reference :default "/Game/ThirdPerson/Input/Actions/IA_Interact.IA_Interact"))
  (bind _follow_camera (Variables|Default|GetFollow%20Camera))
  (bind _returnvalue (Transformation|GetWorldLocation _follow_camera))
  ;[1 1 1] Pick Up Trace
  (:Started
    (bind (_outhit _returnvalue_2) (Collision|SphereTraceForObjects _returnvalue (+ _returnvalue (* (Math|Vector|GetForwardVector (Transformation|GetWorldRotation _follow_camera)) 1e+03)) 15.0 (Utilities|Array|MakeArray "ObjectTypeQuery2") false 0 "ForDuration"))
    (if _returnvalue_2
      (bind _asbp_weapon (Utilities|Casting|CastToBP_Weapon (.HitActor (Collision|BreakHitResult _outhit))))
      (CallFunction|AddWeapon (Variables|/Game/Equipment_System/BP_Weapon.BP_Weapon_C|GetitemData _asbp_weapon))
      (Actor|DestroyActor _asbp_weapon)
      (Development|PrintString "Item Gethered!"))))

(event Input|EnhancedActionEvents|EnhancedInputActionIA_Equipment_Menu
  (params (ActionValue :type Boolean) (ElapsedSeconds :type Float%20%28double-precision%29) (TriggeredSeconds :type Float%20%28double-precision%29) (InputAction :type Input%20Action%20Object%20Reference :default "/Game/ThirdPerson/Input/Actions/IA_Equipment_Menu.IA_Equipment_Menu"))
  (bind _returnvalue (Game|GetPlayerController 0))
  (bind _bpc_attack_system (Variables|Default|GetBPC%20Attack%20System))
  ;[1 1 1] Equipment Menu Panel
  (:Started
    (if (not (Variables|Default|GetisPanelOpened?))
      (Variables|/Game/BluePrints/BPC_AttackSystem.BPC_AttackSystem_C|Setcan%20Attack _bpc_attack_system false)
      (Variables|Default|SetisPanelOpened? true)
      (bind _equipment_widget (Variables|Default|GetEquipment%20Widget)
        (:then
          (Widget|SetVisibility _equipment_widget "Visible"))
        (:else
          (bind _returnvalue_2 (UserInterface|CreateWidget "/Game/Equipment_System/UI/WB_Equipment.WB_Equipment_C"))
          (bind _output_get (Variables|Default|SetEquipment%20Widget _returnvalue_2))
          (UserInterface|Viewport|AddtoViewport _output_get 0)))
      (Variables|/Script/Engine.PlayerController|SetbShowMouseCursor _returnvalue true)
      (Input|SetInputModeGameandUI _returnvalue (Variables|Default|GetEquipment%20Widget) "DoNotLock" true false)
      (bind _asbp_third_person_character (Utilities|Casting|CastToBP_ThirdPersonCharacter (Components|GetOwner)))
      (Pawn|Components|CharacterMovement|SetMovementMode (Variables|/Script/Engine.Character|GetCharacterMovement _asbp_third_person_character) "MOVE_None" 0)
      (else
        (Variables|/Game/BluePrints/BPC_AttackSystem.BPC_AttackSystem_C|Setcan%20Attack _bpc_attack_system true)
        (Variables|Default|SetisPanelOpened? false)
        (bind _equipment_widget_2 (Variables|Default|GetEquipment%20Widget)
          (:then
            (Widget|SetVisibility _equipment_widget_2 "Hidden")
            (Variables|/Script/Engine.PlayerController|SetbShowMouseCursor _returnvalue false)
            (Input|SetInputModeGameOnly _returnvalue false)
            (bind _asbp_third_person_character_2 (Utilities|Casting|CastToBP_ThirdPersonCharacter (Components|GetOwner)))
            (Pawn|Components|CharacterMovement|SetMovementMode (Variables|/Script/Engine.Character|GetCharacterMovement _asbp_third_person_character_2) "MOVE_Walking" 0))
          (:else))))))

(event EventBeginPlay
  (bind _asbp_third_person_character (Utilities|Casting|CastToBP_ThirdPersonCharacter (Components|GetOwner)))
  (Variables|Default|SetFollow%20Camera (Variables|/Game/ThirdPerson/Blueprints/BP_ThirdPersonCharacter.BP_ThirdPersonCharacter_C|GetFollowCamera _asbp_third_person_character))
  (Variables|Default|SetBPC%20Attack%20System (Variables|/Game/ThirdPerson/Blueprints/BP_ThirdPersonCharacter.BP_ThirdPersonCharacter_C|GetBPC_AttackSystem _asbp_third_person_character)))

(event Input|KeyboardEvents|DebugKeyH
  (params (Key :type Key%20Structure :default "None") (ActionValue :type Input%20Action%20Value%20Structure))
  ;[1 1 1] Pick Up Trace
  (:Pressed
    (for _array_element (Variables|Default|GetweaponSlots)
      (Development|PrintString (Utilities|String|ToString(Name) (.rowname (.item _array_element))) true true "(R=0.000000,G=0.660000,B=1.000000,A=1.000000)" 5.0))))

(fn AddWeapon
  (params (NewItem :type S%20Slots%20Structure%20%28by%20ref%29))
  (Utilities|Array|Add (Variables|Default|GetweaponSlots) NewItem))